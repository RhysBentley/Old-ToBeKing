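; BP_CameraController is a top-down style player camera that pans, speeds up, zooms via spring arm, and commands AI characters with the visible cursor.
; Interaction traces under the cursor to select and highlight a BP_CharacterAI, or send the selected one to a BP_Interactive or world point.
; For interactives, a Delay of distance over max speed estimates arrival before turning the character and calling Interact.
; Plain move orders and the Deselect input clear the selection.
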(event `self.ReceiveBeginPlay`
  (bind _returnvalue (`GameplayStatics.GetPlayerController` 0))
  ;[1 1 1] Event Beginplay
  ;;[1 1 1] Showing the cursor
  (`WidgetBlueprintLibrary.SetInputMode_GameAndUIEx` _returnvalue null "DoNotLock" false)
  (set `PlayerController.bShowMouseCursor` true _returnvalue))

(event `InputAxis|MoveForward`
  (params (AxisValue :type "Float (single-precision)"))
  ;[1 1 1] Camera Controls
  ;;[1 1 1] Camera Movement
  (`PawnMovementComponent.AddInputVector` (`self.Movement`) (`KismetMathLibrary.MakeVector` (select `bool` (`self.SpeedUp`) :`false` AxisValue :`true` (* AxisValue 30.0))) false))

(event `InputAxis|MoveRight`
  (params (AxisValue :type "Float (single-precision)"))
  ;[1 1 1] Camera Controls
  ;;[1 1 1] Camera Movement
  (`PawnMovementComponent.AddInputVector` (`self.Movement`) (`KismetMathLibrary.MakeVector` 0.0 (select `bool` (`self.SpeedUp`) :`false` AxisValue :`true` (* AxisValue 30.0))) false))

(event `InputAction|SpeedUp`
  (params (Key :type "Key Structure"))
  (bind _movement (`self.Movement`))
  ;[1 1 1] Camera Controls
  ;;[1 1 1] Speed up Camera Movement
  (:`Pressed`
    (set `self.SpeedUp` true)
    (set `FloatingPawnMovement.MaxSpeed` 2500.0 _movement))
  (:`Released`
    (set `self.SpeedUp` false)
    (set `FloatingPawnMovement.MaxSpeed` 1200.0 _movement)))

(event `InputAxis|ZoomIn/Out`
  (params (AxisValue :type "Float (single-precision)"))
  ;[1 1 1] Camera Controls
  ;;[1 1 1] Zooming in and out
  (set `SpringArmComponent.TargetArmLength` (`KismetMathLibrary.FClamp` (+ (* AxisValue 50.0) (`SpringArmComponent.TargetArmLength` (`self.SpringArm`))) 500.0 2000.0) (`self.SpringArm`)))

(event `InputAction|Interaction`
  (params (Key :type "Key Structure"))
  (bind (_hitresult _returnvalue) (`PlayerController.GetHitResultUnderCursorForObjects` (`GameplayStatics.GetPlayerController` 0) (`|MakeArray` "ObjectTypeQuery7" :!type "EObjectTypeQuery Enum") true))
  (bind (_bblockinghit _binitialoverlap _time _distance _location _impactpoint _normal _impactnormal _physmat _hitactor) (`GameplayStatics.BreakHitResult` (`PlayerController.GetHitResultUnderCursorForObjects` (`GameplayStatics.GetPlayerController` 0) (`|MakeArray` "ObjectTypeQuery1" :!type "EObjectTypeQuery Enum") true)))
  ;[1 1 1] Selecting system
  ;;[1 1 1] Selecting the character
  (:`Pressed`
    (if _returnvalue
      (bind _asbp_character_ai (cast `/Game/Blueprints/CharacterAI/BP_CharacterAI` (`.HitActor` (`GameplayStatics.BreakHitResult` _hitresult)))) ; Selecting the character
      (bind _output_get (set `self.SelectedCharacter` _asbp_character_ai))
      (`/Game/Blueprints/CharacterAI/BP_CharacterAI.Highlight` _output_get true)
      (else
        (bind _asbp_interactive (cast `/Game/Blueprints/InteractiveObjects/BP_Interactive` _hitactor)
          (:`then`
            (bind _selectedcharacter (`self.SelectedCharacter`)
              (:`then`
                (bind _returnvalue_2 (`SceneComponent.K2_GetComponentLocation` (`/Game/Blueprints/InteractiveObjects/BP_Interactive.StaticMesh` _asbp_interactive)))
                (`/Game/Blueprints/CharacterAI/BP_CharacterAI.MoveCharacter` _selectedcharacter _returnvalue_2)
                (`KismetSystemLibrary.Delay` (/ (`KismetMathLibrary.Vector_Distance` (`SceneComponent.K2_GetComponentLocation` (`Character.CapsuleComponent` _selectedcharacter)) _returnvalue_2) (`MovementComponent.GetMaxSpeed` (`Character.CharacterMovement` _selectedcharacter)))) ; Waiting for the character to reach the point
                (bind (_returnvalue_roll _returnvalue_pitch _returnvalue_yaw) (`KismetMathLibrary.BreakRotator` (`KismetMathLibrary.FindLookAtRotation` (`SceneComponent.K2_GetComponentLocation` (`Character.CapsuleComponent` (`self.SelectedCharacter`))) (`SceneComponent.K2_GetComponentLocation` (`/Game/Blueprints/InteractiveObjects/BP_Interactive.StaticMesh` _asbp_interactive)))))
                (`SceneComponent.K2_SetWorldRotation` (`Character.CapsuleComponent` (`self.SelectedCharacter`)) (`KismetMathLibrary.MakeRotator` 0.0 0.0 (+ _returnvalue_yaw -90.0)) false false) ; Rotating to face the object
                (`/Game/Blueprints/InteractiveObjects/BP_Interactive.Interact` _asbp_interactive))
              (:`else`)))
          (:`CastFailed`
            (bind _selectedcharacter_2 (`self.SelectedCharacter`)
              (:`then`
                (`/Game/Blueprints/CharacterAI/BP_CharacterAI.MoveCharacter` _selectedcharacter_2 _location)
                (`self.Deselect`))
              (:`else`))))))))

(event `InputAction|Deselect`
  (params (Key :type "Key Structure"))
  ;[1 1 1] Selecting system
  ;;[1 1 1] Deselecting the character
  (:`Pressed`
    (bind _selectedcharacter (`self.SelectedCharacter` :!label _label)
      (:`then`
        (`/Game/Blueprints/CharacterAI/BP_CharacterAI.Highlight` _selectedcharacter false)
        (set `self.SelectedCharacter` null))
      (:`else`))))

(event `Deselect`
  ;[1 1 1] Selecting system
  ;;[1 1 1] Deselecting the character
  (goto _label))

(fn `UserConstructionScript`)