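; BP_CharacterAI is a base AI character that can be selected through the camera controller pawn and sent to a location.
; MoveCharacter writes the target to the MoveToLocation blackboard key on its AI controller.
; Tick polls the camera controller's SelectedCharacter, sets Highlighted and temporarily tints a construction-script dynamic body material red or grey.
; BeginPlay caches the camera controller and calls Init, which re-applies the Health and Armour statistics unchanged.
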(event `self.ReceiveBeginPlay`
  ;[1 1 1] Event Beginplay
  ;;[1 1 1] Getting reference
  (bind _asbp_camera_controller (cast `/Game/Blueprints/PlayerControlled/BP_CameraController` (`GameplayStatics.GetPlayerPawn` 0)))
  (set `self.CameraControlledReference` _asbp_camera_controller)
  (`self.Init`) ; Setting base information
)

(event `MoveCharacter`
  (params (MoveToLocation :type "Vector Structure"))
  ;[1 1 1] Moving the character to a given location
  (bind _asbp_character_aicontroller (cast `/Game/Blueprints/CharacterAI/Base/BP_CharacterAIController` (`AIBlueprintHelperLibrary.GetAIController` self)))
  (`BlackboardComponent.SetValueAsVector` (`/Game/Blueprints/CharacterAI/Base/BP_CharacterAIController.Blackboard Component` _asbp_character_aicontroller) "MoveToLocation" MoveToLocation))

(event `self.ReceiveTick`
  (params (DeltaSeconds :type "Float (single-precision)"))
  (bind _dmi_skeletal (`self.DMI_Skeletal`))
  ;[1 1 1] Highlighting the character
  (if (== (`/Game/Blueprints/PlayerControlled/BP_CameraController.SelectedCharacter` (`self.CameraControlledReference`)) self)
    (set `self.Highlighted` true)
    (`MaterialInstanceDynamic.SetVectorParameterValue` _dmi_skeletal "BodyColour" (struct :`R` 1.0 :`A` 1.0)) ; Temp
    (else
      (set `self.Highlighted` false)
      (`MaterialInstanceDynamic.SetVectorParameterValue` _dmi_skeletal "BodyColour" (struct :`R` 0.5 :`G` 0.5 :`B` 0.5 :`A` 1.0)) ; Temp
    )))

(fn `Init`
  (bind _statistics (`self.Statistics`))
  (bind (_health _maxhealth _armour) (break `/Game/Structures/Struct_Statistics` _statistics))
  (setmembers `/Game/Structures/Struct_Statistics` :`StructRef` _statistics :`Health` _health :`Armour` _armour))

(fn `UserConstructionScript`
  (bind _returnvalue (`PrimitiveComponent.CreateDynamicMaterialInstance` (`self.Mesh`) 0 "/Game/Mannequin/Character/Materials/M_Male_Body.M_Male_Body" "None"))
  (set `self.DMI_Skeletal` _returnvalue))